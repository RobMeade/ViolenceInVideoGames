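; BP_SaveGame is the save game object that persists GameMetrics to a named save slot.
; Initialise sets the metrics in memory, while SaveData stores them and writes the object to the slot.
; LoadData copies metrics from an existing save into this instance, or creates the slot from the current instance if none exists, then returns them.
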(fn `Initialise`
  (params (GameMetrics :type "Array of /Game/VIG/Core/Structures/SGameMetrics Structure"))
  ;[1 1 1] Initialise
  (set `self._GameMetrics` GameMetrics))

(fn `LoadData`
  (returns (GameMetrics :type "Array of /Game/VIG/Core/Structures/SGameMetrics Structure"))
  ;[1 1 1] Load Data
  (bind _returnvalue (`GameplayStatics.DoesSaveGameExist` (`self._SlotName`)))
  (if _returnvalue
    (bind _returnvalue_2 (`GameplayStatics.LoadGameFromSlot` (`self._SlotName`)))
    (bind _asbp_save_game (cast `/Game/VIG/Core/SaveGame/BP_SaveGame` _returnvalue_2))
    (set `self._GameMetrics` (`/Game/VIG/Core/SaveGame/BP_SaveGame._GameMetrics` _asbp_save_game))
    (else
      (`GameplayStatics.SaveGameToSlot` self (`self._SlotName`))))
  (return (`self._GameMetrics`)))

(fn `SaveData`
  (params (GameMetrics :type "Array of /Game/VIG/Core/Structures/SGameMetrics Structure"))
  ;[1 1 1] Save Data
  (set `self._GameMetrics` GameMetrics)
  (`GameplayStatics.SaveGameToSlot` self (`self._SlotName`)))