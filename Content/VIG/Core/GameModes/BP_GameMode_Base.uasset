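; Base game mode that runs a play session, from input-locked introduction through timed play to completion and return to MainMenu.
; It picks the play mode from the "Game" URL option, registers with the game instance and responds to player controller intro, pause and completion events.
; A timeline drives the game timer, and the final time goes into the controller's metrics.
; Registered blocks and NPCs have their destruction re-broadcast through its dispatchers.
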(event `self.ReceiveBeginPlay`
  ;[1 1 1] Initialise
  (`self.SetPlayModeFromGameOptions`)
  (`self.SetReferences`)
  (`self.BindToEvents`)
  (`self.RegisterWithGameInstance`)
  (`self.DisablePlayerInput`))

(event `StartGameTimer`
  ;[1 1 1] Game Timer
  (bind (_direction _delta) (`Timeline|GameTimer` :!via `PlayFromStart` :!label _label)
    (:`Update`
      (`self.IncrementGameTimer` (* _delta (`GameplayStatics.GetWorldDeltaSeconds`))))))

(event `StopGameTimer`
  ;[1 1 1] Game Timer
  (goto _label :!via `Stop`))

(event `self.ReceiveEndPlay`
  (params (EndPlayReason :type "EEndPlayReason Enum" :default "Destroyed"))
  ;[1 1 1] Finalise
  (`self.UnbindAllEvents`))

(fn `BindToEvents`
  ;[1 1 1] Bind to Events
  (add `/Game/VIG/Core/Characters/Player/BP_PlayerController.PlayerPauseGameToggled` (`self._PlayerController`) (`|CreateDelegate` :!event `OnPlayerPauseGameToggled`))
  (add `/Game/VIG/Core/Characters/Player/BP_PlayerController.PlayModeCompleted` (`self._PlayerController`) (`|CreateDelegate` :!event `OnPlayModeCompleted`))
  (add `/Game/VIG/Core/Characters/Player/BP_PlayerController.PlayModeIntroductionBeginButtonClicked` (`self._PlayerController`) (`|CreateDelegate` :!event `OnPlayModeIntroductionBeginButtonClicked`)))

(fn `DisablePlayerInput`
  (bind __playercontroller (`self._PlayerController`))
  ;[1 1 1] Disable Player Input
  (`self.DisableInput` __playercontroller __playercontroller))

(fn `GetEnabledMechanics`
  (returns (EnabledMechanics :type "/Game/VIG/Core/Structures/SEnabledMechanics Structure"))
  ;[1 1 1] Get Enabled Mechanics
  (return (`self._EnabledMechanics`)))

(fn `GetGameInstance`
  (returns (GameInstance :type "/Game/VIG/Core/BP_GameInstance Object Reference"))
  ;[1 1 1] Get Game Instance
  (return (`self._GameInstance`)))

(fn `GetPlayerController`
  (returns (PlayerController :type "/Game/VIG/Core/Characters/Player/BP_PlayerController Object Reference"))
  ;[1 1 1] Get Player Controller
  (return (`self._PlayerController`)))

(fn `GetPlayMode`
  (returns (PlayMode :type "/Game/VIG/Core/Enum/EPlayMode Enum"))
  ;[1 1 1] Get Play Mode
  (return (`self._PlayMode`)))

(fn `IncrementGameTimer`
  (params (Delta :type "Float (double-precision)"))
  ;[1 1 1] Increment Game Timer
  (bind _output_get (set `self._GameTime` (+ (`self._GameTime`) Delta)))
  (`self.GameTimerUpdated` _output_get))

(fn `OnBlockDestroyed`
  (params (DestructionSource :type "/Game/VIG/Core/Enum/EDestructionSource Enum" :default "NewEnumerator0"))
  ;[1 1 1] Block Destroyed
  (`self.BlockDestroyed` DestructionSource))

(fn `OnNPCDestroyed`
  ;[1 1 1] NPC Destroyed
  (`self.NPCDestroyed`))

(fn `OnPlayerPauseGameToggled`
  ;[1 1 1] Player Pause Game Toggled
  (`GameplayStatics.SetGamePaused` (not (`GameplayStatics.IsGamePaused`)))
  (`/Game/VIG/Core/Characters/Player/BP_PlayerController.ToggleGamePaused` (`self._PlayerController`) (`GameplayStatics.IsGamePaused`)))

(fn `OnPlayModeCompleted`
  ;[1 1 1] Play Mode Completed
  (`self.StopGameTimer`)
  (`/Game/VIG/Core/Characters/Player/BP_PlayerController.FinaliseGameMetrics` (`self._PlayerController`) (`self._GameTime`))
  (`self.PlayModeCompleted` (`/Game/VIG/Core/Characters/Player/BP_PlayerController.GetGameMetrics` (`self._PlayerController`)))
  (`GameplayStatics.OpenLevel` "MainMenu"))

(fn `OnPlayModeIntroductionBeginButtonClicked`
  (bind __playercontroller (`self._PlayerController`))
  ;[1 1 1] Play Mode Introduction Begin Button Clicked
  (`self.StartGameTimer`)
  (`self.EnableInput` __playercontroller __playercontroller))

(fn `RegisterBlock`
  (params (Block :type "/Game/VIG/Core/Characters/Player/BP_Block Object Reference"))
  ;[1 1 1] Register Block
  (add `/Game/VIG/Core/Characters/Player/BP_Block.Destroyed` Block (`|CreateDelegate` :!event `OnBlockDestroyed`)))

(fn `RegisterNPC`
  (params (NPC :type "/Game/VIG/Core/Characters/NPC/BP_NPC Object Reference"))
  ;[1 1 1] Register NPC
  (add `/Game/VIG/Core/Characters/NPC/BP_NPC.Destroyed` NPC (`|CreateDelegate` :!event `OnNPCDestroyed`)))

(fn `RegisterWithGameInstance`
  ;[1 1 1] Register with Game Instance
  (`/Game/VIG/Core/BP_GameInstance.Register` (`self._GameInstance`) self))

(fn `ResetEnvironment`
  ;[1 1 1] Reset Environment
  (bind _outactors (`GameplayStatics.GetAllActorsOfClass` "/Game/VIG/Core/Characters/Player/BP_Block.BP_Block_C"))
  (`self.K2_DestroyActor` _outactors))

(fn `SetEnabledMechanics`
  (params (EnabledMechanics :type "/Game/VIG/Core/Structures/SEnabledMechanics Structure"))
  ;[1 1 1] Set Enabled Mechanics
  (set `self._EnabledMechanics` EnabledMechanics))

(fn `SetPlayModeFromGameOptions`
  (locals (_CurrentPlayMode :type "/Game/VIG/Core/Enum/EPlayMode Enum"))
  ;[1 1 1] Set Play Mode from Game Options
  (bind _enumvalue (foreach `/Game/VIG/Core/Enum/EPlayMode` false)
    (:`LoopBody`
      (bind _output_get (set `local._CurrentPlayMode` _enumvalue))
      (if (== (`|GetEnumeratorNameAsString` _output_get) (`GameplayStatics.ParseOption` (`self.OptionsString`) "Game"))
        (set `self._PlayMode` (`local._CurrentPlayMode`))))))

(fn `SetReferences`
  ;[1 1 1] Set References
  (bind _asbp_game_instance (cast `/Game/VIG/Core/BP_GameInstance` (`GameplayStatics.GetGameInstance`)))
  (set `self._GameInstance` _asbp_game_instance)
  (bind _asbp_player_controller (cast `/Game/VIG/Core/Characters/Player/BP_PlayerController` (`GameplayStatics.GetPlayerController` 0)))
  (set `self._PlayerController` _asbp_player_controller))

(fn `UnbindAllEvents`
  ;[1 1 1] Unbind All Events
  (clear `self.BlockDestroyed`)
  (clear `self.GameTimerUpdated`)
  (clear `self.NPCDestroyed`)
  (clear `self.PlayModeCompleted`))

(fn `UserConstructionScript`)