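; Paper2D NPC that patrols horizontally around its spawn point, starting in a random direction and registering with the game mode.
; Each tick it moves along X, turning around at its movement range or after overlapping a non-player actor, with a flag preventing repeated flips.
; A short forward object trace halts movement and snaps the NPC to the 100-unit grid horizontally.
; Its Destroy event fires the Destroyed dispatcher before removing the actor.
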(event `self.ReceiveBeginPlay`
  ;[1 1 1] Initialise
  (`self.SetRandomForwardDirection`)
  (`self.SetOrigin`)
  (`self.RegisterWithGameMode`))

(event `self.ReceiveTick`
  (params (DeltaSeconds :type "Float (single-precision)"))
  ;[1 1 1] Tick
  (`self.MoveHorizontally` DeltaSeconds))

(event `self.ReceiveEndPlay`
  (params (EndPlayReason :type "EEndPlayReason Enum" :default "Destroyed"))
  ;[1 1 1] Finalise
  (`self.UnbindAllEvents`))

(event `self.PaperFlipbook.OnComponentBeginOverlap`
  (params (OverlappedComponent :type "PrimitiveComponent Object Reference") (OtherActor :type "Actor Object Reference") (OtherComp :type "PrimitiveComponent Object Reference") (OtherBodyIndex :type Integer) (bFromSweep :type Boolean) (SweepResult :type "HitResult Structure (by ref)"))
  ;[1 1 1] Change Horizontal Direction
  (`self.SetMustChangeDirection` OtherActor))

(event `/Game/VIG/Core/Interfaces/BPI_Destroyable.Destroy`
  (params (DestructionSource :type "/Game/VIG/Core/Enum/EDestructionSource Enum" :default "NewEnumerator0"))
  ;[1 1 1] Self Destruct
  (`self.SelfDestruct`))

(fn `ChangeHorizontalDirection`
  (bind _returnvalue_x (`KismetMathLibrary.BreakVector` (`self.GetActorForwardVector`)))
  (bind (_returnvalue_roll _returnvalue_pitch _returnvalue_yaw) (`KismetMathLibrary.BreakRotator` (`SceneComponent.K2_GetComponentRotation` (`self.Scene`))))
  (`SceneComponent.K2_SetWorldRotation` (`self.Scene`) (`KismetMathLibrary.MakeRotator` 0.0 0.0 (+ _returnvalue_yaw (* _returnvalue_x 180.0))) false false)
  (`self.SetCanMove`)
  (set `self._HasChangedDirection` true)
  (set `self._MustChangeDirection` false))

(fn `GetGridPositionLocation`
  (returns (Location :type "Vector Structure"))
  (bind (_returnvalue_x _returnvalue_y _returnvalue_z) (`KismetMathLibrary.BreakVector` (`self.K2_GetActorLocation`)))
  ;[1 1 1] Get Grid Position Location
  (return (`KismetMathLibrary.MakeVector` (- (* (`KismetMathLibrary.FCeil` (/ _returnvalue_x 100.0)) 100.0) 50.0) 0.0 (* (/ _returnvalue_z 100.0) 100.0))))

(fn `GetLineTraceSegment`
  (returns (Start :type "Vector Structure") (End :type "Vector Structure"))
  (bind _returnvalue (`self.K2_GetActorLocation`))
  ;[1 1 1] Get Line Trace
  (return _returnvalue (+ _returnvalue (* (`self.GetActorForwardVector`) (50.0 0.0 0.0)))))

(fn `GetMoveLocation`
  (params (DeltaSeconds :type "Float (double-precision)"))
  (returns (Location :type "Vector Structure"))
  (bind (_returnvalue_x _returnvalue_y _returnvalue_z) (`KismetMathLibrary.BreakVector` (`self.K2_GetActorLocation`)))
  (bind _returnvalue_x_2 (`KismetMathLibrary.BreakVector` (`self.GetActorForwardVector`)))
  ;[1 1 1] Get Move Location
  (return (`KismetMathLibrary.MakeVector` (+ (* (`local.DeltaSeconds`) (`self.Speed`) _returnvalue_x_2) _returnvalue_x) _returnvalue_y _returnvalue_z)))

(fn `HasReachedMovementRange`
  (returns (ReturnValue :type Boolean))
  (bind _returnvalue_x (`KismetMathLibrary.BreakVector` (`self.K2_GetActorLocation`)))
  (bind _returnvalue_x_2 (`KismetMathLibrary.BreakVector` (`self.K2_GetActorLocation`)))
  (bind __origin_x (`KismetMathLibrary.BreakVector` (`self._Origin`)))
  (bind __origin_x_2 (`KismetMathLibrary.BreakVector` (`self._Origin`)))
  (return (or (>= _returnvalue_x_2 (+ __origin_x (`self.MovementRange`))) (<= _returnvalue_x (- __origin_x_2 (`self.MovementRange`))))))

(fn `MoveHorizontally`
  (params (DeltaSeconds :type "Float (double-precision)"))
  ;[1 1 1] Move Horizontally
  (if (or (`self._MustChangeDirection`) (`self.HasReachedMovementRange`))
    (if (`self._HasChangedDirection`)
      (`self.SetCanMove`)
      (set `self._MustChangeDirection` false)
      (if (`self._CanMove`) :!label _label
        (`self.K2_SetActorLocation` (`self.GetMoveLocation` (`local.DeltaSeconds`))))
      (else
        (`self.ChangeHorizontalDirection`)))
    (else
      (`self.SetCanMove`)
      (set `self._HasChangedDirection` false)
      (goto _label))))

(fn `RegisterWithGameMode`
  ;[1 1 1] Register with Game Mode
  (bind _asbp_game_mode_base (cast `/Game/VIG/Core/GameModes/BP_GameMode_Base` (`GameplayStatics.GetGameMode`)))
  (`/Game/VIG/Core/GameModes/BP_GameMode_Base.RegisterNPC` _asbp_game_mode_base self))

(fn `SelfDestruct`
  ;[1 1 1] Self Destruct
  (`self.Destroyed`)
  (`self.K2_DestroyActor`))

(fn `SetCanMove`
  (locals (GridPositionX :type "Float (double-precision)") (GridPositionZ :type "Float (double-precision)"))
  (bind (_start _end) (`self.GetLineTraceSegment`))
  ;[1 1 1] Set Can Move
  (bind (_outhit _returnvalue) (`KismetSystemLibrary.LineTraceSingleForObjects` :`Start` _start :`End` _end :`ObjectTypes` (`|MakeArray` "ObjectTypeQuery8" :!type "EObjectTypeQuery Enum") :`DrawTime` 2.0))
  (if _returnvalue
    (set `self._CanMove` false)
    (`self.K2_SetActorLocation` (`self.GetGridPositionLocation`))
    (else
      (set `self._CanMove` true))))

(fn `SetMustChangeDirection`
  (params (OtherActor :type "Actor Object Reference"))
  ;[1 1 1] Set Mush Change Direction
  (set `self._MustChangeDirection` (!= (`GameplayStatics.GetObjectClass` OtherActor) "/Game/VIG/Core/Characters/Player/BP_PlayerCharacter.BP_PlayerCharacter_C")))

(fn `SetOrigin`
  ;[1 1 1] Set Origin
  (set `self._Origin` (`self.K2_GetActorLocation`)))

(fn `SetRandomForwardDirection`
  ;[1 1 1] Set Random Forward Direction
  (`self.K2_SetActorRotation` (select `bool` (`KismetMathLibrary.RandomBool`) :`true` (struct :`Yaw` 180.0) :!type "Rotator Structure")))

(fn `UnbindAllEvents`
  ;[1 1 1] Unbind All Events
  (clear `self.Destroyed`))

(fn `UserConstructionScript`)