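; Player projectile that travels horizontally and destroys what it hits.
; Each tick it moves along X by Speed and the X of its set Direction, without sweeping, so hits come from overlap events.
; Overlapping the tile map destroys it; actors implementing BPI_Destroyable also receive a destroy message first, and others are ignored.
; It broadcasts its Destroyed dispatcher before removal and clears those bindings on EndPlay.
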(event `self.ReceiveTick`
  (params (DeltaSeconds :type "Float (single-precision)"))
  ;[1 1 1] Tick
  (`self.Move` DeltaSeconds))

(event `self.ReceiveEndPlay`
  (params (EndPlayReason :type "EEndPlayReason Enum" :default "Destroyed"))
  ;[1 1 1] Finalise
  (clear `self.Destroyed`))

(event `self.Projectile.OnComponentBeginOverlap`
  (params (OverlappedComponent :type "PrimitiveComponent Object Reference") (OtherActor :type "Actor Object Reference") (OtherComp :type "PrimitiveComponent Object Reference") (OtherBodyIndex :type Integer) (bFromSweep :type Boolean) (SweepResult :type "HitResult Structure (by ref)"))
  ;[1 1 1] Collision
  (`self.Collide` OtherActor))

(fn `Collide`
  (params (OtherActor :type "Actor Object Reference"))
  ;[1 1 1] Collide
  (if (== (`GameplayStatics.GetObjectClass` OtherActor) "/Game/VIG/Environment/BP_TileMap.BP_TileMap_C")
    (`self.SelfDestruct`)
    (elif (`KismetSystemLibrary.DoesImplementInterface` (`local.OtherActor`) "/Game/VIG/Core/Interfaces/BPI_Destroyable.BPI_Destroyable_C")
      (message `/Game/VIG/Core/Interfaces/BPI_Destroyable.Destroy` (`local.OtherActor`) "NewEnumerator1")
      (`self.SelfDestruct`))))

(fn `Move`
  (params (DeltaSeconds :type "Float (double-precision)"))
  (bind (_returnvalue_x _returnvalue_y _returnvalue_z) (`KismetMathLibrary.BreakVector` (`self.K2_GetActorLocation`)))
  (bind __direction_x (`KismetMathLibrary.BreakVector` (`self._Direction`)))
  ;[1 1 1] Move
  (`self.K2_SetActorLocation` (`KismetMathLibrary.MakeVector` (+ (* (* DeltaSeconds (`self._Speed`)) __direction_x) _returnvalue_x) _returnvalue_y _returnvalue_z)))

(fn `SelfDestruct`
  ;[1 1 1] Self Destruct
  (`self.Destroyed`)
  (`self.K2_DestroyActor`))

(fn `SetDirection`
  (params (Direction :type "Vector Structure"))
  ;[1 1 1] Set Direction
  (set `self._Direction` Direction))

(fn `UserConstructionScript`)