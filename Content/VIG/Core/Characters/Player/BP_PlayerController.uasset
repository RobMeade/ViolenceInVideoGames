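; Player controller for a side-scrolling game with jumping, shooting and block building across multiple play modes.
; Relays input to the character, gating build, fire and reset by GameMode's enabled mechanics, and snaps yaw to horizontal travel direction.
; Creates menu, admin and play-mode widgets, handling their events, level changes and input modes.
; Tallies player actions and game events into a metrics struct, and re-enables firing when the registered projectile is destroyed.
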(event `self.ReceiveBeginPlay`
  ;[1 1 1] Initialise
  (`self.SetReferences`)
  (`self.BindToGameEvents`))

(event `self.ReceiveTick`
  (params (DeltaSeconds :type "Float (single-precision)"))
  ;[1 1 1] Tick
  (if (`self._InputEnabled`)
    (`self.UpdateControlRotation`)))

(event `self.ReceiveEndPlay`
  (params (EndPlayReason :type "EEndPlayReason Enum" :default "Destroyed"))
  ;[1 1 1] Finalise
  (`self.UnbindAllEvents`))

(event `InputAction|Jump`
  (params (Key :type "Key Structure"))
  ;[1 1 1] Player Interaction
  (:`Pressed`
    (`self.JumpStart`)
    (`self.UpdateGameMetrics` "NewEnumerator2"))
  (:`Released`
    (`self.JumpStop`)))

(event `InputAxis|MoveRight`
  (params (AxisValue :type "Float (single-precision)"))
  ;[1 1 1] Player Interaction
  (`self.MoveHorizontally` AxisValue)
  (`/Engine/EditorBlueprintResources/StandardMacros.CompareFloat` AxisValue
    (:`>`
      (`/Engine/EditorBlueprintResources/StandardMacros.DoOnce` false :!label _label
        (:`Completed`
          (`self.UpdateGameMetrics` "NewEnumerator1")
          (goto _label_2 :!via `Reset`))))
    (:`==`
      (`|ExecutionSequence`
        (:`then_0`
          (goto _label :!via `Reset`))
        (:`then_1`
          (goto _label_2 :!via `Reset`))))
    (:`<`
      (`/Engine/EditorBlueprintResources/StandardMacros.DoOnce` false :!label _label_2
        (:`Completed`
          (`self.UpdateGameMetrics` "NewEnumerator0")
          (goto _label :!via `Reset`))))))

(event `InputAction|ToggleBuildMode`
  (params (Key :type "Key Structure"))
  ;[1 1 1] Player Interaction
  (:`Pressed`
    (`self.ToggleBuildMode`)))

(event `InputAction|CreateBlock`
  (params (Key :type "Key Structure"))
  (bind _enabledmechanics_createblocks (break `/Game/VIG/Core/Structures/SEnabledMechanics` (`/Game/VIG/Core/GameModes/BP_GameMode_Base.GetEnabledMechanics` (`self._GameMode`))))
  ;[1 1 1] Player Interaction
  (:`Pressed`
    (if _enabledmechanics_createblocks
      (`self.Create`))))

(event `InputAction|ResetEnvironment`
  (params (Key :type "Key Structure"))
  (bind (_enabledmechanics_createblocks _enabledmechanics_destroyblocks _enabledmechanics_fire _enabledmechanics_resetenvironment) (break `/Game/VIG/Core/Structures/SEnabledMechanics` (`/Game/VIG/Core/GameModes/BP_GameMode_Base.GetEnabledMechanics` (`self._GameMode`))))
  ;[1 1 1] Player Interaction
  (:`Pressed`
    (if _enabledmechanics_resetenvironment
      (`/Game/VIG/Core/GameModes/BP_GameMode_Base.ResetEnvironment` (`self._GameMode`))
      (`self.UpdateGameMetrics` "NewEnumerator7"))))

(event `InputAction|DestroyBlock`
  (params (Key :type "Key Structure"))
  (bind (_enabledmechanics_createblocks _enabledmechanics_destroyblocks) (break `/Game/VIG/Core/Structures/SEnabledMechanics` (`/Game/VIG/Core/GameModes/BP_GameMode_Base.GetEnabledMechanics` (`self._GameMode`))))
  ;[1 1 1] Player Interaction
  (:`Pressed`
    (if _enabledmechanics_destroyblocks
      (`self.Destroy`))))

(event `InputAction|Fire`
  (params (Key :type "Key Structure"))
  (bind (_enabledmechanics_createblocks _enabledmechanics_destroyblocks _enabledmechanics_fire) (break `/Game/VIG/Core/Structures/SEnabledMechanics` (`/Game/VIG/Core/GameModes/BP_GameMode_Base.GetEnabledMechanics` (`self._GameMode`))))
  ;[1 1 1] Player Interaction
  (:`Pressed`
    (if _enabledmechanics_fire
      (if (`self._CanFire`)
        (set `self._CanFire` false)
        (`/Game/VIG/Core/Characters/Player/BP_PlayerCharacter.Fire` (`self._PlayerCharacter`))
        (`self.UpdateGameMetrics` "NewEnumerator5")))))

(event `InputAction|TogglePauseGame` :paused true
  (params (Key :type "Key Structure"))
  ;[1 1 1] Player Interaction
  (:`Pressed`
    (`self.PlayerPauseGameToggled`)))

(fn `BindToAdminUIEvents`
  ;[1 1 1] Bind to Admin Events
  (add `/Game/VIG/UI/WBP_Admin.MainMenuButtonClicked` (`self._UIAdminWidget`) (`|CreateDelegate` :!event `OnAdminMainMenuButtonClicked`)))

(fn `BindToGameEvents`
  ;[1 1 1] Bind to Game Events
  (add `/Game/VIG/Core/GameModes/BP_GameMode_Base.GameTimerUpdated` (`self._GameMode`) (`|CreateDelegate` :!event `OnGameTimerUpdated`))
  (add `/Game/VIG/Core/GameModes/BP_GameMode_Base.NPCDestroyed` (`self._GameMode`) (`|CreateDelegate` :!event `OnNPCDestroyed`))
  (add `/Game/VIG/Core/GameModes/BP_GameMode_Base.BlockDestroyed` (`self._GameMode`) (`|CreateDelegate` :!event `OnBlockDestroyed`)))

(fn `BindToGameUIEvents`
  ;[1 1 1] Bind to Game UI Events
  (add `/Game/VIG/UI/WBP_PlayModeIntroduction.PlayModeIntroductionBeginButtonClicked` (`self._UIPlayModeIntroductionWidget`) (`|CreateDelegate` :!event `OnPlayModeIntroductionBeginButtonClicked`))
  (add `/Game/VIG/UI/WBP_GamePaused.GamePausedResumeButtonClicked` (`self._UIGamePausedWidget`) (`|CreateDelegate` :!event `OnGamePausedResumeButtonClicked`))
  (add `/Game/VIG/UI/WBP_PlayModeComplete.PlayModeCompleteContinueBeginButtonClicked` (`self._UIPlayModeCompleteWidget`) (`|CreateDelegate` :!event `OnPlayModeCompleteContinueButtonClicked`)))

(fn `BindToMainMenuUIEvents`
  ;[1 1 1] Bind to UI Events
  (add `/Game/VIG/UI/WBP_MainMenu.PlayModeButtonClicked` (`self._UIMainMenuWidget`) (`|CreateDelegate` :!event `OnMainMenuGameModeButtonClicked`))
  (add `/Game/VIG/UI/WBP_MainMenu.QuitButtonClicked` (`self._UIMainMenuWidget`) (`|CreateDelegate` :!event `OnMainMenuQuitButtonClicked`))
  (add `/Game/VIG/UI/WBP_MainMenu.AdminButtonClicked` (`self._UIMainMenuWidget`) (`|CreateDelegate` :!event `OnMainMenuAdminButtonClicked`)))

(fn `Create`
  ;[1 1 1] Create Block
  (if (`self._InputEnabled`)
    (if (`self._BuildModeEnabled`)
      (`/Game/VIG/Core/Characters/Player/BP_PlayerCharacter.Create` (`self._PlayerCharacter`)))))

(fn `CreateUIWidgetsForAdmin`
  ;[1 1 1] Create UI Widgets for Admin
  (bind _returnvalue (`|CreateWidget` "/Game/VIG/UI/WBP_Admin.WBP_Admin_C" self))
  (bind _output_get (set `self._UIAdminWidget` _returnvalue))
  (`UserWidget.AddToViewport` _output_get 0))

(fn `CreateUIWidgetsForGame`
  (params (PlayMode :type "/Game/VIG/Core/Enum/EPlayMode Enum" :default "NewEnumerator4"))
  ;[1 1 1] Create UI Widgets for Game
  (bind _returnvalue (`|CreateWidget` "/Game/VIG/UI/WBP_PlayModeIntroduction.WBP_PlayModeIntroduction_C" self))
  (bind _output_get (set `self._UIPlayModeIntroductionWidget` _returnvalue))
  (`UserWidget.AddToViewport` _output_get 0)
  (bind _returnvalue_2 (`|CreateWidget` "/Game/VIG/UI/WBP_GamePaused.WBP_GamePaused_C" self))
  (bind _output_get_2 (set `self._UIGamePausedWidget` _returnvalue_2))
  (`UserWidget.AddToViewport` _output_get_2 0)
  (`Widget.SetVisibility` (`self._UIGamePausedWidget`) "Hidden")
  (bind _returnvalue_3 (`|CreateWidget` "/Game/VIG/UI/WBP_PlayModeComplete.WBP_PlayModeComplete_C" self))
  (bind _output_get_3 (set `self._UIPlayModeCompleteWidget` _returnvalue_3))
  (`UserWidget.AddToViewport` _output_get_3 0)
  (`Widget.SetVisibility` (`self._UIPlayModeCompleteWidget`) "Hidden")
  (`self.SetInputModeUIOnly` null))

(fn `CreateUIWidgetsForMainMenu`
  ;[1 1 1] Create UI Widgets for Menu
  (bind _returnvalue (`|CreateWidget` "/Game/VIG/UI/WBP_MainMenu.WBP_MainMenu_C" self))
  (bind _output_get (set `self._UIMainMenuWidget` _returnvalue))
  (`UserWidget.AddToViewport` _output_get 0))

(fn `Destroy`
  ;[1 1 1] Destroy Block
  (if (`self._InputEnabled`)
    (if (`self._BuildModeEnabled`)
      (`/Game/VIG/Core/Characters/Player/BP_PlayerCharacter.Destroy` (`self._PlayerCharacter`)))))

(fn `DetermineHorizontalDirectionOfMovement`
  (params (AxisValue :type "Float (double-precision)"))
  ;[1 1 1] Determine Direction of Movement
  (`/Engine/EditorBlueprintResources/StandardMacros.CompareFloat` AxisValue
    (:`>`
      (set `self._IsMovingRight` true))
    (:`<`
      (set `self._IsMovingRight` false))))

(fn `FinaliseGameMetrics`
  (params (GameTime :type "Float (double-precision)"))
  ;[1 1 1] Finalise Game Metrics
  (setmembers `/Game/VIG/Core/Structures/SGameMetrics` :`StructRef` (`self._GameMetrics`) :`GameDuration` GameTime))

(fn `GetGameMetrics`
  (returns (GameMetrics :type "/Game/VIG/Core/Structures/SGameMetrics Structure"))
  ;[1 1 1] Get Game Metrics
  (return (`self._GameMetrics`)))

(fn `GetHorizontalVelocity`
  (returns (Velocity :type "Float (double-precision)"))
  (bind _velocity_x (`KismetMathLibrary.BreakVector` (`MovementComponent.Velocity` (`Pawn.GetMovementComponent` (`self._PlayerCharacter`)))))
  ;[1 1 1] Get Horizontal Velocity
  (return _velocity_x))

(fn `GetLevelByPlayMode`
  (params (PlayMode :type "/Game/VIG/Core/Enum/EPlayMode Enum" :default "NewEnumerator0"))
  (returns (LevelName :type Name) (Options :type String))
  (bind _returnvalue (`|GetEnumeratorNameAsString` PlayMode))
  ;[1 1 1] Get Level by Play Mode
  (return (`KismetStringLibrary.Conv_StringToName` (`KismetStringLibrary.Concat_StrStr` "Game_" _returnvalue)) (`KismetStringLibrary.Concat_StrStr` "Game=" _returnvalue)))

(fn `InitialiseForAdmin`
  (params (GameMetrics :type "Array of /Game/VIG/Core/Structures/SGameMetrics Structure"))
  ;[1 1 1] Initialise for Admin
  (`self.CreateUIWidgetsForAdmin`)
  (`self.BindToAdminUIEvents`)
  (`self.SetInputModeUIOnly` (`self._UIAdminWidget`))
  (`/Game/VIG/UI/WBP_Admin.Initialise` (`self._UIAdminWidget`) (`local.GameMetrics`)))

(fn `InitialiseForGame`
  (params (PlayMode :type "/Game/VIG/Core/Enum/EPlayMode Enum (by ref)"))
  ;[1 1 1] Initialise - Game
  (`self.InitialiseGameMetrics` PlayMode)
  (`self.CreateUIWidgetsForGame` (`local.PlayMode`))
  (`self.BindToGameUIEvents`)
  (`/Game/VIG/UI/WBP_PlayModeIntroduction.Initialise` (`self._UIPlayModeIntroductionWidget`) (`local.PlayMode`)))

(fn `InitialiseForMainMenu`
  (params (ActivePlayMode :type "/Game/VIG/Core/Enum/EPlayMode Enum" :default "NewEnumerator4"))
  ;[1 1 1] Initialise - Main Menu
  (`self.CreateUIWidgetsForMainMenu`)
  (`self.BindToMainMenuUIEvents`)
  (`self.SetInputModeUIOnly` (`self._UIMainMenuWidget`))
  (`/Game/VIG/UI/WBP_MainMenu.ActivatePlayMode` (`self._UIMainMenuWidget`) (`local.ActivePlayMode`)))

(fn `InitialiseGameMetrics`
  (params (PlayMode :type "/Game/VIG/Core/Enum/EPlayMode Enum (by ref)"))
  ;[1 1 1] Initialise Game Metrics
  (setmembers `/Game/VIG/Core/Structures/SGameMetrics` :`StructRef` (`self._GameMetrics`) :`DateTime` (`KismetMathLibrary.Now`) :`PlayMode` PlayMode))

(fn `JumpStart`
  ;[1 1 1] Jump - Start
  (`/Game/VIG/Core/Characters/Player/BP_PlayerCharacter.JumpStart` (`self._PlayerCharacter`)))

(fn `JumpStop`
  ;[1 1 1] Jump - Stop
  (`/Game/VIG/Core/Characters/Player/BP_PlayerCharacter.JumpStop` (`self._PlayerCharacter`)))

(fn `MoveHorizontally`
  (params (AxisValue :type "Float (double-precision)"))
  ;[1 1 1] Move Horizontally
  (if (`self._InputEnabled`)
    (`self.DetermineHorizontalDirectionOfMovement` (`local.AxisValue`))
    (`/Game/VIG/Core/Characters/Player/BP_PlayerCharacter.MoveRight` (`self._PlayerCharacter`) (`local.AxisValue`))))

(fn `OnAdminMainMenuButtonClicked`
  ;[1 1 1] Admin - Main Menu Button Clicked
  (`GameplayStatics.OpenLevel` "MainMenu"))

(fn `OnBlockCreated`
  ;[1 1 1] Block Created
  (`self.UpdateGameMetrics` "NewEnumerator3"))

(fn `OnBlockDestroyed`
  (params (DestructionSource :type "/Game/VIG/Core/Enum/EDestructionSource Enum" :default "NewEnumerator0"))
  ;[1 1 1] Block Destroyed
  (`self.UpdateGameMetrics` (select `/Game/VIG/Core/Enum/EDestructionSource` DestructionSource :`NewEnumerator0` "NewEnumerator4" :`NewEnumerator1` "NewEnumerator10" :!type "/Game/VIG/Core/Enum/EPlayerEventDataType Enum")))

(fn `OnGamePausedResumeButtonClicked`
  ;[1 1 1] Game Paused Resume Button Clicked
  (`self.PlayerPauseGameToggled`))

(fn `OnGameTimerUpdated`
  (params (GameTime :type "Float (double-precision)"))
  ;[1 1 1] Game Timer Updated
  (`/Game/VIG/Core/BP_HUD.UpdateGameTimer` (`self._HUD`) GameTime))

(fn `OnGoalReached`
  ;[1 1 1] Goal Reached
  (set `self._InputEnabled` false)
  (`self.UpdateGameMetrics` "NewEnumerator9")
  (`self.PlayModeCompleted`)
  (`Widget.SetVisibility` (`self._UIPlayModeCompleteWidget`) "SelfHitTestInvisible")
  (`/Game/VIG/UI/WBP_PlayModeComplete.Initialise` (`self._UIPlayModeCompleteWidget`) (`/Game/VIG/Core/GameModes/BP_GameMode_Base.GetPlayMode` (`self._GameMode`)))
  (`self.SetInputModeUIOnly` null))

(fn `OnMainMenuAdminButtonClicked`
  ;[1 1 1] Main Menu - Admin Button Clicked
  (`GameplayStatics.OpenLevel` "Admin" true "Game=Admin"))

(fn `OnMainMenuGameModeButtonClicked`
  (params (Mode :type "/Game/VIG/Core/Enum/EPlayMode Enum" :default "NewEnumerator0"))
  (bind (_levelname _options) (`self.GetLevelByPlayMode` Mode))
  ;[1 1 1] Main Menu - Game Mode Button Clicked
  (`GameplayStatics.OpenLevel` _levelname true _options))

(fn `OnMainMenuQuitButtonClicked`
  ;[1 1 1] Main Menu - Quit Button Clicked
  (clear `self.PlayerPauseGameToggled`)
  (`KismetSystemLibrary.QuitGame` null "Quit"))

(fn `OnNPCDestroyed`
  ;[1 1 1] NPC Destroyed
  (`self.UpdateGameMetrics` "NewEnumerator6"))

(fn `OnPlayModeCompleteContinueButtonClicked`
  ;[1 1 1] Play Mode Complete Continue Button Clicked
  (`Widget.SetVisibility` (`self._UIPlayModeCompleteWidget`) "Hidden")
  (`GameplayStatics.OpenLevel` "MainMenu"))

(fn `OnPlayModeIntroductionBeginButtonClicked`
  ;[1 1 1] Play Mode Introduction Begin Button Clicked
  (`Widget.SetVisibility` (`self._UIPlayModeIntroductionWidget`) "Hidden")
  (`/Game/VIG/Core/BP_HUD.SetGameTimerVisibility` (`self._HUD`) "SelfHitTestInvisible")
  (`self.SetInputModeGameOnly`)
  (`self.PlayModeIntroductionBeginButtonClicked`))

(fn `OnProjectileDestroyed`
  ;[1 1 1] Projectile Destroyed
  (set `self._CanFire` true))

(fn `RegisterCharacter`
  (params (PlayerCharacter :type "/Game/VIG/Core/Characters/Player/BP_PlayerCharacter Object Reference"))
  ;[1 1 1] Register
  (set `self._PlayerCharacter` PlayerCharacter)
  (add `/Game/VIG/Core/Characters/Player/BP_PlayerCharacter.BlockCreated` (`self._PlayerCharacter`) (`|CreateDelegate` :!event `OnBlockCreated`))
  (add `/Game/VIG/Core/Characters/Player/BP_PlayerCharacter.BlockDestroyed` (`self._PlayerCharacter`) (`|CreateDelegate` :!event `OnBlockDestroyed`))
  (add `/Game/VIG/Core/Characters/Player/BP_PlayerCharacter.GoalReached` (`self._PlayerCharacter`) (`|CreateDelegate` :!event `OnGoalReached`))
  (set `self._InputEnabled` true))

(fn `RegisterProjectile`
  (params (Projectile :type "/Game/VIG/Core/Characters/Player/BP_Projectile Object Reference"))
  ;[1 1 1] Register Projectile
  (add `/Game/VIG/Core/Characters/Player/BP_Projectile.Destroyed` Projectile (`|CreateDelegate` :!event `OnProjectileDestroyed`)))

(fn `SetInputModeGameOnly`
  ;[1 1 1] Set Input Mode - Game Only
  (`WidgetBlueprintLibrary.SetInputMode_GameOnly` self)
  (set `self.bShowMouseCursor` false))

(fn `SetInputModeUIOnly`
  (params (WidgetToFocus :type "Widget Object Reference"))
  ;[1 1 1] Set Input Mode - UI Only
  (`WidgetBlueprintLibrary.SetInputMode_UIOnlyEx` self WidgetToFocus)
  (set `self.bShowMouseCursor` true))

(fn `SetReferences`
  ;[1 1 1] Set References
  (bind _asbp_game_mode_base (cast `/Game/VIG/Core/GameModes/BP_GameMode_Base` (`GameplayStatics.GetGameMode`)))
  (set `self._GameMode` _asbp_game_mode_base)
  (bind _asbp_hud (cast `/Game/VIG/Core/BP_HUD` (`self.GetHUD`)))
  (set `self._HUD` _asbp_hud))

(fn `ToggleBuildMode`
  ;[1 1 1] Toggle Build Mode
  (if (`self._InputEnabled`)
    (set `self._BuildModeEnabled` (not (`self._BuildModeEnabled`)))
    (`/Game/VIG/Core/Characters/Player/BP_PlayerCharacter.ToggleBuildMode` (`self._PlayerCharacter`) (`self._BuildModeEnabled`))))

(fn `ToggleGamePaused`
  (params (Paused :type Boolean))
  ;[1 1 1] Toggle Game Paused
  (if Paused
    (`Widget.SetVisibility` (`self._UIGamePausedWidget`) "SelfHitTestInvisible")
    (`WidgetBlueprintLibrary.SetInputMode_GameAndUIEx` self null)
    (set `self.bShowMouseCursor` true)
    (else
      (`Widget.SetVisibility` (`self._UIGamePausedWidget`) "Hidden")
      (`WidgetBlueprintLibrary.SetInputMode_GameOnly` self)
      (set `self.bShowMouseCursor` false))))

(fn `UnbindAllEvents`
  ;[1 1 1] Unbind All Events
  (clear `self.PlayerPauseGameToggled`)
  (clear `self.PlayModeCompleted`)
  (clear `self.PlayModeIntroductionBeginButtonClicked`))

(fn `UpdateControlRotation`
  ;[1 1 1] Update Control Rotation
  (bind _velocity (`self.GetHorizontalVelocity`))
  (`/Engine/EditorBlueprintResources/StandardMacros.CompareFloat` _velocity
    (:`>`
      (`self.SetControlRotation` (`KismetMathLibrary.MakeRotator` 0.0) :!label _label))
    (:`==`
      (if (`self._IsMovingRight`)
        (goto _label)
        (else
          (`self.SetControlRotation` (`KismetMathLibrary.MakeRotator` 0.0 0.0 180.0) :!label _label_2))))
    (:`<`
      (goto _label_2))))

(fn `UpdateGameMetrics`
  (params (PlayerEvent :type "/Game/VIG/Core/Enum/EPlayerEventDataType Enum" :default "NewEnumerator0"))
  (bind (__gamemetrics_datetime __gamemetrics_playmode __gamemetrics_playermovedleft __gamemetrics_playermovedright __gamemetrics_playerjumped __gamemetrics_playerfired __gamemetrics_npcsdestroyed __gamemetrics_blocksplaced __gamemetrics_blocksdestroyedbuildtool __gamemetrics_blocksdestroyedprojectile __gamemetrics_resetenvironment __gamemetrics_gamequit __gamemetrics_goalreached) (break `/Game/VIG/Core/Structures/SGameMetrics` (`self._GameMetrics`)))
  ;[1 1 1] Update Game Metrics
  (`/Engine/EditorBlueprintResources/StandardMacros.IncrementInt` (select `/Game/VIG/Core/Enum/EPlayerEventDataType` PlayerEvent :`NewEnumerator0` __gamemetrics_playermovedleft :`NewEnumerator1` __gamemetrics_playermovedright :`NewEnumerator2` __gamemetrics_playerjumped :`NewEnumerator5` __gamemetrics_playerfired :`NewEnumerator6` __gamemetrics_npcsdestroyed :`NewEnumerator3` __gamemetrics_blocksplaced :`NewEnumerator4` __gamemetrics_blocksdestroyedbuildtool :`NewEnumerator10` __gamemetrics_blocksdestroyedprojectile :`NewEnumerator7` __gamemetrics_resetenvironment :`NewEnumerator8` __gamemetrics_gamequit :`NewEnumerator9` __gamemetrics_goalreached)))

(fn `UserConstructionScript`)