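; Falling block actor that registers itself with BP_GameMode_Base and drops until it lands on a surface.
; Each tick it traces downward until a hit sets a rounded landing point, otherwise targeting one trace length lower, and starts falling.
; The Fall timeline moves it toward that target with constant interpolation at a steadily rising speed, then fires Landed.
; Destruction broadcasts Destroyed with its source, unbinds both dispatchers and removes the actor.
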(event `self.ReceiveBeginPlay`
  ;[1 1 1] Initialise
  (bind _asbp_game_mode_base (cast `/Game/VIG/Core/GameModes/BP_GameMode_Base` (`GameplayStatics.GetGameMode`)))
  (`/Game/VIG/Core/GameModes/BP_GameMode_Base.RegisterBlock` _asbp_game_mode_base self))

(event `self.ReceiveTick`
  (params (DeltaSeconds :type "Float (single-precision)"))
  ;[1 1 1] Tick
  (`self.LineTraceForCollision`))

(event `self.ReceiveEndPlay`
  (params (EndPlayReason :type "EEndPlayReason Enum" :default "Destroyed"))
  ;[1 1 1] Finalise
  (`self.UnbindAllEvents`))

(event `FallBegin`
  ;[1 1 1] Manage Fall
  (bind (_direction _alpha) (`Timeline|Fall` :!via `PlayFromStart` :!label _label)
    (:`Update`
      (`self.MoveBlock` _alpha))))

(event `FallEnd`
  ;[1 1 1] Manage Fall
  (goto _label :!via `Stop`))

(event `/Game/VIG/Core/Interfaces/BPI_Destroyable.Destroy`
  (params (DestructionSource :type "/Game/VIG/Core/Enum/EDestructionSource Enum" :default "NewEnumerator0"))
  ;[1 1 1] Destroy Block
  (`self.SelfDestruct` DestructionSource))

(fn `GetLineTraceStartAndEnd`
  (returns (Start :type "Vector Structure") (End :type "Vector Structure"))
  (bind _returnvalue (+ (`self.K2_GetActorLocation`) (50.0 0.0 0.0)))
  ;[1 1 1] Get Line Trace Start and End
  (return _returnvalue (`KismetMathLibrary.MakeVector` (.x _returnvalue) (.y _returnvalue) (- (.z _returnvalue) (`self._LineTraceLength`)))))

(fn `GetMoveToLocationFromHitLocation`
  (params (InVec :type "Vector Structure"))
  (returns (ReturnValue :type "Vector Structure"))
  ;[1 1 1] Get MoveTo Location from Hit Location
  (return (`KismetMathLibrary.MakeVector` (- (.x InVec) 50.0) 0.0 (`KismetMathLibrary.Conv_IntToDouble` (`KismetMathLibrary.Round` (.z InVec))))))

(fn `LineTraceForCollision`
  (locals (Hit :type "HitResult Structure"))
  (bind (_start _end) (`self.GetLineTraceStartAndEnd`))
  (bind (_hit_bblockinghit _hit_binitialoverlap _hit_time _hit_distance _hit_location) (`GameplayStatics.BreakHitResult` (`local.Hit`)))
  ;[1 1 1] Line Trace for Collision
  (if (not (`self._HasFallTarget`))
    (bind (_outhit _returnvalue) (`KismetSystemLibrary.LineTraceSingle` _start _end "TraceTypeQuery1"))
    (set `local.Hit` _outhit)
    (if _returnvalue
      (if _hit_bblockinghit
        (set `self._HasFallTarget` true)
        (set `self._MoveTo` (`self.GetMoveToLocationFromHitLocation` _hit_location))
        (if (not (`self._IsFalling`)) :!label _label
          (`self.FallBegin`)
          (set `self._IsFalling` true)))
      (else
        (set `self._MoveTo` (- (`self.K2_GetActorLocation`) (`KismetMathLibrary.MakeVector` 0.0 0.0 (`self._LineTraceLength`))))
        (goto _label)))))

(fn `MoveBlock`
  (params (Alpha :type "Float (double-precision)"))
  (bind (_returnvalue_x _returnvalue_y _returnvalue_z) (`KismetMathLibrary.BreakVector` (`self.K2_GetActorLocation`)))
  (bind (__moveto_x __moveto_y __moveto_z) (`KismetMathLibrary.BreakVector` (`self._MoveTo`)))
  ;[1 1 1] Move Block
  (`self.K2_SetActorLocation` (`KismetMathLibrary.VInterpTo_Constant` (`self.K2_GetActorLocation`) (`self._MoveTo`) Alpha (`self._FallSpeed`)))
  (if (<= _returnvalue_z __moveto_z)
    (set `self._IsFalling` false)
    (`self.FallEnd`)
    (`self.Landed`)
    (else
      (set `self._FallSpeed` (+ (`self._FallSpeed`) 1.0)))))

(fn `SelfDestruct`
  (params (DestructionSource :type "/Game/VIG/Core/Enum/EDestructionSource Enum" :default "NewEnumerator0"))
  ;[1 1 1] Self Destruct
  (`self.Destroyed` DestructionSource)
  (clear `self.Landed`)
  (clear `self.Destroyed`)
  (`self.K2_DestroyActor`))

(fn `UnbindAllEvents`
  ;[1 1 1] Unbind All Events
  (clear `self.Destroyed`)
  (clear `self.Landed`))

(fn `UserConstructionScript`)